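; BP_floortile is a map tile for a side-scroller that extends the level as the player runs through it.
; When a SideScroller3Character hits EndTrigger, the tile has MySideScroller3GameMode add the next tile, then destroys itself after a delay.
; Its construction script randomizes content only on the server to avoid client mismatches, spawning child actors as a blocker or coins.
; An upper-blocker branch exists, but the current random range never selects it.
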(event `self.EndTrigger.OnComponentBeginOverlap`
  (params (OverlappedComponent :type "PrimitiveComponent Object Reference") (OtherActor :type "Actor Object Reference") (OtherComp :type "PrimitiveComponent Object Reference") (OtherBodyIndex :type Integer) (bFromSweep :type Boolean) (SweepResult :type "HitResult Structure (by ref)"))
  ;[1 1 1] エンドトリガーと接触後、マップ（BP_floortile）を生成。
  ; 始めのマップはゲームモードのbeginにて生成される
  (cast `SideScroller3Character` OtherActor)
  (bind _asmy_side_scroller_3game_mode (cast `/Game/SakaiNew/MySideScroller3GameMode` (`GameplayStatics.GetGameMode`)))
  (`/Game/SakaiNew/MySideScroller3GameMode.AddFloorTile` _asmy_side_scroller_3game_mode)
  (`KismetSystemLibrary.Delay` 7.0)
  (`self.K2_DestroyActor`))

(fn `GetAttackPoint`
  (returns (AttachPoint :type "Transform Structure"))
  (return (`SceneComponent.K2_GetComponentToWorld` (`self.AttackPoint`))))

(fn `SetSpawnPoint`
  (set `self.SpawnPoints` (`|MakeArray` (`SceneComponent.GetRelativeTransform` (`self.SpawnPoint`)) (`SceneComponent.GetRelativeTransform` (`self.SpawnPoint2`)) (`SceneComponent.GetRelativeTransform` (`self.SpawnPoint3`)))))

(fn `SpawnBlocker`
  (bind _spawnpoints (`self.SpawnPoints`))
  (`AddComponent|NODE_AddChildActorComponent-0` :`RelativeTransform` (`|GetArrayItem` _spawnpoints (`KismetMathLibrary.RandomIntegerInRange` 0 (`KismetArrayLibrary.Array_LastIndex` _spawnpoints)))))

(fn `SpawnCoins`
  (bind _coinarea (`self.CoinArea`))
  (for _ (range (+ (`KismetMathLibrary.RandomIntegerInRange` 0 5) 1))
    (`AddComponent|NODE_AddChildActorComponent-1` :`RelativeTransform` (`KismetMathLibrary.Conv_VectorToTransform` (`KismetMathLibrary.RandomPointInBoundingBox` (`SceneComponent.RelativeLocation` _coinarea) (`BoxComponent.BoxExtent` _coinarea))))))

(fn `SpawnUpBlocker`
  (bind _upblockarea (`self.UpBlockArea`))
  (`AddComponent|NODE_AddChildActorComponent-2` :`RelativeTransform` (`KismetMathLibrary.Conv_VectorToTransform` (`KismetMathLibrary.RandomPointInBoundingBox` (`SceneComponent.RelativeLocation` _upblockarea) (`BoxComponent.BoxExtent` _upblockarea)))))

(fn `UserConstructionScript`
  ;[1 1 1] サーバーでのみ、障害物、アイテムなどを生成する
  ; サーバーでのみ実行しないとクライアントで別の乱数が振られてしまう。
  (if (`KismetSystemLibrary.IsServer`)
    (`self.SetSpawnPoint`)
    (switch `int` (`KismetMathLibrary.RandomIntegerInRange` 2 3)
      (:`Default`
        (`self.SpawnBlocker` :!label _label))
      (:`0`
        (goto _label))
      (:`1`
        (`self.SpawnUpBlocker`))
      (:`2`
        (`self.SpawnCoins`)))))